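; Player controller for moving the current cube in fixed steps with the arrow keys, with Escape quitting the game.
; On BeginPlay it caches BP_GameInstance and shows the WB_Menu widget unless Restart is set.
; Each arrow key runs a short Visibility line trace from the GameInstance's Current actor and, if nothing is hit, teleports that actor a longer step that way.
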(event EventBeginPlay
  (bind _asbp_game_instance (Utilities|Casting|CastToBP_GameInstance (Game|GetGameInstance)))
  (Variables|Default|SetGame%20Instance _asbp_game_instance)
  (if (not (Variables|Default|GetRestart?))
    (bind _returnvalue (UserInterface|CreateWidget "/Game/Blueprints/interface/WB_Menu.WB_Menu_C" self))
    (bind _output_get (Variables|Default|SetWB_Menu _returnvalue))
    (UserInterface|Viewport|AddtoViewport _output_get 0)))

(event Input|KeyboardEvents|Escape
  (params (Key :type Key%20Structure :default "None"))
  (:Pressed
    (Game|QuitGame 0 "Quit" false)))

(event Input|KeyboardEvents|Right
  (params (Key :type Key%20Structure :default "None"))
  (:Pressed
    (bind _returnvalue (CallFunction|LineTracebyChannel "0.000000,200.000000, 0"))
    (if (not _returnvalue)
      (CallFunction|CubeConrolled "0.000000,300.000000, 0"))))

(event Input|KeyboardEvents|Up
  (params (Key :type Key%20Structure :default "None"))
  (:Pressed
    (bind _returnvalue (CallFunction|LineTracebyChannel "200.000000, 0, 0"))
    (if (not _returnvalue)
      (CallFunction|CubeConrolled "300.000000, 0, 0"))))

(event Input|KeyboardEvents|Down
  (params (Key :type Key%20Structure :default "None"))
  (:Pressed
    (bind _returnvalue (CallFunction|LineTracebyChannel "-200.000000, 0, 0"))
    (if (not _returnvalue)
      (CallFunction|CubeConrolled "-300.000000, 0, 0"))))

(event Input|KeyboardEvents|Left
  (params (Key :type Key%20Structure :default "None"))
  (:Pressed
    (bind _returnvalue (CallFunction|LineTracebyChannel "0.000000,-200.000000, 0"))
    (if (not _returnvalue)
      (CallFunction|CubeConrolled "0.000000,-300.000000, 0"))))

(fn ConstructionScript)

(fn CubeConrolled
  (params (B :type Vector))
  (bind _game_instance (Variables|Default|GetGame%20Instance))
  (bind _current (Variables|/Game/Blueprints/PuzzleSystem/BP_GameInstance.BP_GameInstance_C|GetCurrent _game_instance))
  (Transformation|SetActorLocation _current (+ (Transformation|GetActorLocation _current) B) false true))

(fn LineTracebyChannel
  (params (B :type Vector))
  (bind _game_instance (Variables|Default|GetGame%20Instance))
  (bind _current (Variables|/Game/Blueprints/PuzzleSystem/BP_GameInstance.BP_GameInstance_C|GetCurrent _game_instance))
  (bind _returnvalue (Transformation|GetActorLocation _current))
  (Utilities|IsValid _current
    (:Is%20Valid
      (bind _returnvalue_2 (Collision|LineTraceByChannel (+ _returnvalue "0, 0,5.000000") (+ (+ _returnvalue B) "0, 0,5.000000") "TraceTypeQuery1" true 0 "None" true "(R=1.000000,G=0.000000,B=0.000000,A=1.000000)" "(R=0.000000,G=1.000000,B=0.000000,A=1.000000)" 3.0))
      (return _returnvalue_2))))