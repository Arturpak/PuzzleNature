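; BP_Grid is the board of a color-sorting puzzle, won by filling red, orange and yellow columns with matching cubes.
; Each column's collision tracks overlapping BP_Cubes of its color, marking it complete at five and clearing it when one leaves.
; Completing all three shows the WB_End widget, while Tick mirrors that state into Finish.
; BeginPlay snaps the grid to a fixed position, then raises it after a short delay.
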(event OnComponentBeginOverlap(CollisionRed)
  (params (OverlappedComponent :type Primitive%20Component%20Object%20Reference) (OtherActor :type Actor%20Object%20Reference) (OtherComp :type Primitive%20Component%20Object%20Reference) (OtherBodyIndex :type Integer) (bFromSweep :type Boolean) (SweepResult :type Hit%20Result%20Structure%20%28by%20ref%29))
  (bind _checkupmassivred (Variables|Default|GetCheckupMassivRed))
  (bind _asbp_cube (Utilities|Casting|CastToBP_Cube OtherActor))
  (if (Utilities|Enum|Equal(Enum) (Variables|/Game/Blueprints/PuzzleSystem/BP_Cube.BP_Cube_C|GetColorCube _asbp_cube) "NewEnumerator0")
    (Utilities|Array|AddUnique _checkupmassivred _asbp_cube)
    (if (== (Utilities|Array|Length _checkupmassivred) 5)
      (bind _output_get (Variables|Default|SetRedСolumn%20 true))
      (if (Math|Boolean|ANDBoolean _output_get (stale OnComponentBeginOverlap(CollisionOrange) _output_get) (stale OnComponentBeginOverlap(CollisionYellow) _output_get))
        (bind _returnvalue (UserInterface|CreateWidget "/Game/Blueprints/interface/WB_End.WB_End_C" (Game|GetPlayerController 0)))
        (bind _output_get_2 (Variables|Default|SetWB_End _returnvalue))
        (UserInterface|Viewport|AddtoViewport _output_get_2 0)))))

(event OnComponentEndOverlap(CollisionRed)
  (params (OverlappedComponent :type Primitive%20Component%20Object%20Reference) (OtherActor :type Actor%20Object%20Reference) (OtherComp :type Primitive%20Component%20Object%20Reference) (OtherBodyIndex :type Integer))
  (bind _asbp_cube (Utilities|Casting|CastToBP_Cube OtherActor))
  (if (Utilities|Enum|Equal(Enum) (Variables|/Game/Blueprints/PuzzleSystem/BP_Cube.BP_Cube_C|GetColorCube _asbp_cube) "NewEnumerator0")
    (Utilities|Array|RemoveItem (Variables|Default|GetCheckupMassivRed) _asbp_cube)
    (Variables|Default|SetRedСolumn%20 false)))

(event OnComponentBeginOverlap(CollisionOrange)
  (params (OverlappedComponent :type Primitive%20Component%20Object%20Reference) (OtherActor :type Actor%20Object%20Reference) (OtherComp :type Primitive%20Component%20Object%20Reference) (OtherBodyIndex :type Integer) (bFromSweep :type Boolean) (SweepResult :type Hit%20Result%20Structure%20%28by%20ref%29))
  (bind _checkupmassivorange (Variables|Default|GetCheckupMassivOrange))
  (bind _asbp_cube (Utilities|Casting|CastToBP_Cube OtherActor))
  (if (Utilities|Enum|Equal(Enum) (Variables|/Game/Blueprints/PuzzleSystem/BP_Cube.BP_Cube_C|GetColorCube _asbp_cube) "NewEnumerator2")
    (Utilities|Array|AddUnique _checkupmassivorange _asbp_cube)
    (if (== (Utilities|Array|Length _checkupmassivorange) 5)
      (bind _output_get (Variables|Default|SetOrangeСolumn%20 true))
      (if (Math|Boolean|ANDBoolean (stale OnComponentBeginOverlap(CollisionRed) _output_get) _output_get (stale OnComponentBeginOverlap(CollisionYellow) _output_get))
        (bind _returnvalue (UserInterface|CreateWidget "/Game/Blueprints/interface/WB_End.WB_End_C" (Game|GetPlayerController 0)))
        (bind _output_get_2 (Variables|Default|SetWB_End _returnvalue))
        (UserInterface|Viewport|AddtoViewport _output_get_2 0)))))

(event OnComponentEndOverlap(CollisionOrange)
  (params (OverlappedComponent :type Primitive%20Component%20Object%20Reference) (OtherActor :type Actor%20Object%20Reference) (OtherComp :type Primitive%20Component%20Object%20Reference) (OtherBodyIndex :type Integer))
  (bind _asbp_cube (Utilities|Casting|CastToBP_Cube OtherActor))
  (if (Utilities|Enum|Equal(Enum) (Variables|/Game/Blueprints/PuzzleSystem/BP_Cube.BP_Cube_C|GetColorCube _asbp_cube) "NewEnumerator2")
    (Utilities|Array|RemoveItem (Variables|Default|GetCheckupMassivOrange) _asbp_cube)
    (Variables|Default|SetOrangeСolumn%20 false)))

(event OnComponentBeginOverlap(CollisionYellow)
  (params (OverlappedComponent :type Primitive%20Component%20Object%20Reference) (OtherActor :type Actor%20Object%20Reference) (OtherComp :type Primitive%20Component%20Object%20Reference) (OtherBodyIndex :type Integer) (bFromSweep :type Boolean) (SweepResult :type Hit%20Result%20Structure%20%28by%20ref%29))
  (bind _checkupmassivyellow (Variables|Default|GetCheckupMassivYellow))
  (bind _asbp_cube (Utilities|Casting|CastToBP_Cube OtherActor))
  (if (Utilities|Enum|Equal(Enum) (Variables|/Game/Blueprints/PuzzleSystem/BP_Cube.BP_Cube_C|GetColorCube _asbp_cube) "NewEnumerator1")
    (Utilities|Array|AddUnique _checkupmassivyellow _asbp_cube)
    (if (== (Utilities|Array|Length _checkupmassivyellow) 5)
      (bind _output_get (Variables|Default|SetYellowСolumn%20 true))
      (if (Math|Boolean|ANDBoolean (stale OnComponentBeginOverlap(CollisionRed) _output_get) (stale OnComponentBeginOverlap(CollisionOrange) _output_get) _output_get)
        (bind _returnvalue (UserInterface|CreateWidget "/Game/Blueprints/interface/WB_End.WB_End_C" (Game|GetPlayerController 0)))
        (bind _output_get_2 (Variables|Default|SetWB_End _returnvalue))
        (UserInterface|Viewport|AddtoViewport _output_get_2 0)))))

(event OnComponentEndOverlap(CollisionYellow)
  (params (OverlappedComponent :type Primitive%20Component%20Object%20Reference) (OtherActor :type Actor%20Object%20Reference) (OtherComp :type Primitive%20Component%20Object%20Reference) (OtherBodyIndex :type Integer))
  (bind _asbp_cube (Utilities|Casting|CastToBP_Cube OtherActor))
  (if (Utilities|Enum|Equal(Enum) (Variables|/Game/Blueprints/PuzzleSystem/BP_Cube.BP_Cube_C|GetColorCube _asbp_cube) "NewEnumerator1")
    (Utilities|Array|RemoveItem (Variables|Default|GetCheckupMassivYellow) _asbp_cube)
    (Variables|Default|SetYellowСolumn%20 false)))

(event EventBeginPlay
  (bind _defaultsceneroot (Variables|Default|GetDefaultSceneRoot))
  (Transformation|SetWorldLocation _defaultsceneroot "-290.000000,-600.000000,-260.000000" false false)
  (Utilities|FlowControl|Delay 1.0)
  (Transformation|SetWorldLocation _defaultsceneroot "-290.000000,-600.000000,-140.000000" false false))

(event EventTick
  (params (DeltaSeconds :type Float%20%28single-precision%29))
  (if (Math|Boolean|ANDBoolean (Variables|Default|GetRedСolumn%20) (Variables|Default|GetOrangeСolumn%20) (Variables|Default|GetYellowСolumn%20))
    (Variables|Default|SetFinish? true)
    (else
      (Variables|Default|SetFinish? false))))

(fn ConstructionScript)

(fn CheckColor
  (params (Array :type Array%20of%20BP%20Cube%20Object%20References) (Format :type Text) (TextColor :type Linear%20Color%20Structure))
  (for _array_element Array
    (Development|PrintString (Utilities|GetDisplayName _array_element) true true TextColor 0.0))
  (Development|PrintString (Utilities|String|ToString(Text) (Utilities|Text|FormatText Format)) true true TextColor 0.0)
  (return))