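; BP_Cube is a clickable puzzle cube whose color type sets its fire, earth or water mesh and matching material in the construction script.
; On BeginPlay it caches all cubes in the level and writes itself to BP_GameInstance.
; A click resets any active cube's material and scale, then marks the clicked cube active, stretches it in height and stores it as the GameInstance's Current selection.
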(event OnClicked(Cube)
  (params (TouchedComponent :type Primitive%20Component%20Object%20Reference) (ButtonPressed :type Key%20Structure :default "None"))
  (for _array_element (Variables|Default|GetArrayCubes)
    (if (Variables|BP_Cube_C|GetActivate _array_element)
      (Rendering|Material|SetMaterial (Variables|BP_Cube_C|GetCube _array_element) 0 (Utilities|Select :Index (Variables|BP_Cube_C|GetColorCube _array_element) :NewEnumerator0 "/Game/Blueprints/Materials/MI_Red.MI_Red" :NewEnumerator1 "/Game/Blueprints/Materials/MI_Yellow.MI_Yellow" :NewEnumerator2 "/Game/Blueprints/Materials/MI_Orange.MI_Orange"))
      (Variables|BP_Cube_C|SetActivate _array_element false)
      (Development|PrintString "ДеактивированЫЫЫЫ")
      (Transformation|SetRelativeScale3D (Variables|BP_Cube_C|GetCube _array_element) "2.000000,2.000000,0.500000")
      (Variables|/Game/Blueprints/PuzzleSystem/BP_GameInstance.BP_GameInstance_C|SetCurrent (Variables|Default|GetGameInstance) 0)))
  (if (Variables|Default|GetActivate)
    (Transformation|SetRelativeScale3D (Variables|BP_Cube_C|GetCube (Variables|Default|GetCurrent)) "2.000000,2.000000,0.500000")
    (Variables|/Game/Blueprints/PuzzleSystem/BP_GameInstance.BP_GameInstance_C|SetCurrent (Variables|Default|GetGameInstance) 0)
    (Development|PrintString "Очищено" true true "(R=0.000000,G=0.660000,B=1.000000,A=1.000000)" 5.0)
    (Variables|Default|SetActivate false)
    (else
      (bind _output_get (Variables|/Game/Blueprints/PuzzleSystem/BP_GameInstance.BP_GameInstance_C|SetCurrent (Variables|Default|GetGameInstance) self))
      (Development|PrintString (Utilities|GetDisplayName _output_get))
      (Transformation|SetRelativeScale3D (Variables|BP_Cube_C|GetCube _output_get) "2.000000,2.000000,1.300000")
      (Variables|Default|SetActivate true))))

(event EventBeginPlay
  (bind _outactors (Actor|GetAllActorsOfClass "BP_Cube_C"))
  (Variables|Default|SetArrayCubes _outactors)
  (bind _asbp_game_instance (Utilities|Casting|CastToBP_GameInstance (Game|GetGameInstance)))
  (bind _output_get (Variables|Default|SetGameInstance _asbp_game_instance))
  (Variables|/Game/Blueprints/PuzzleSystem/BP_GameInstance.BP_GameInstance_C|SetBP_Cube _output_get self))

(fn ConstructionScript
  (bind _staticmesh (Variables|Default|GetStaticMesh))
  (switch Utilities|FlowControl|Switch|SwitchonE_ColorCube (Variables|Default|GetColorCube)
    (:NewEnumerator0
      (Components|StaticMesh|SetStaticMesh _staticmesh "/Game/Blueprints/Meshes/CubeFire.CubeFire")
      (Variables|Default|SetMaterial "/Game/Blueprints/Materials/MI_Red.MI_Red"))
    (:NewEnumerator1
      (Components|StaticMesh|SetStaticMesh _staticmesh "/Game/Blueprints/Meshes/Cubeearth.Cubeearth")
      (Variables|Default|SetMaterial "/Game/Blueprints/Materials/MI_Yellow.MI_Yellow"))
    (:NewEnumerator2
      (Components|StaticMesh|SetStaticMesh _staticmesh "/Game/Blueprints/Meshes/Cubewater.Cubewater")
      (Variables|Default|SetMaterial "/Game/Blueprints/Materials/MI_Orange.MI_Orange")))
  (Rendering|Material|SetMaterial (Variables|Default|GetCube) 0 (Variables|Default|GetMaterial)))